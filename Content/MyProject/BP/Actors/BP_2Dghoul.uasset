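; 2D ghoul actor that plays out a short visual swap and removes itself once it becomes killable.
; It starts with GhoulIdle visible and Ghoulanim hidden.
; Tick polls IsKillable and BbeKilled, neither set in this graph; when killable and not BbeKilled, it shows Ghoulanim, waits briefly, then hides it and destroys the actor.
; A delayed chain that restores the idle visual is disconnected and never runs.
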(event `self.ReceiveBeginPlay`
  (`SceneComponent.SetVisibility` (`self.GhoulIdle`) true false)
  (`SceneComponent.SetVisibility` (`self.Ghoulanim`) false false))

(event `self.ReceiveTick`
  (params (DeltaSeconds :type "Float (single-precision)"))
  (bind _ghoulanim (`self.Ghoulanim`))
  (if (and (`self.bIsKillable`) (not (`self.bbeKilled`)))
    (`SceneComponent.SetVisibility` (`self.GhoulIdle`) false false)
    (`SceneComponent.SetVisibility` _ghoulanim true false)
    (`KismetSystemLibrary.Delay` 0.5)
    (`SceneComponent.SetVisibility` _ghoulanim false false)
    (`self.K2_DestroyActor`)))

(fn `UserConstructionScript`)